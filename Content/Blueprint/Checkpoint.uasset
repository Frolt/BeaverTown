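; Checkpoint actor that saves the player's progress when touched, marked by a spotlight in a configurable color.
; When MainCharacter_BP overlaps its sphere, it resets health and stores the character's location and an active-checkpoint flag in MainGameInstance_BP.
; It then plays a success sound at the world origin and destroys itself, so each checkpoint triggers once.
; The spotlight color is applied in both the construction script and BeginPlay.
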(event OnComponentBeginOverlap(Sphere)
  (params (OverlappedComponent :type Primitive%20Component%20Object%20Reference) (OtherActor :type Actor%20Object%20Reference) (OtherComp :type Primitive%20Component%20Object%20Reference) (OtherBodyIndex :type Integer) (bFromSweep :type Boolean) (SweepResult :type Hit%20Result%20Structure%20%28by%20ref%29))
  ;[1 1 1] Saves players location when overlapping checkpoint
  (bind _asmain_character_bp (Utilities|Casting|CastToMainCharacter_BP OtherActor))
  (bind _asmain_game_instance_bp (Utilities|Casting|CastToMainGameInstance_BP (Game|GetGameInstance)))
  (Class|MainGameInstance|ResetHealth _asmain_game_instance_bp 1e+02)
  (Variables|/Game/Blueprint/MainGameInstance_BP.MainGameInstance_BP_C|SetPlayerLocation _asmain_game_instance_bp (Transformation|GetActorLocation _asmain_character_bp))
  (Variables|/Game/Blueprint/MainGameInstance_BP.MainGameInstance_BP_C|SetActivateCheckpoint _asmain_game_instance_bp true)
  (Audio|PlaySoundatLocation "/Game/Audio/Success.Success" "0, 0, 0")
  (Actor|DestroyActor))

(event EventBeginPlay
  (Rendering|Components|Light|SetLightColor (Variables|Default|GetSpotLight) (Variables|Default|GetColor) true))

(fn ConstructionScript
  (Rendering|Components|Light|SetLightColor (Variables|Default|GetSpotLight) (Variables|Default|GetColor) true))