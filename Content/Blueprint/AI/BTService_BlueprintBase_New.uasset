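; Behavior tree service that feeds the player's state to AI blackboards.
; On each tick it writes the first player controller's pawn and location to blackboard keys, plus the alive flag read from the MainCharacter cast.
; Without a valid pawn it zeroes the location and clears the player object, leaving the alive key untouched.
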(event EventTick
  (params (OwnerActor :type Actor%20Object%20Reference) (DeltaSeconds :type Float%20%28single-precision%29))
  (bind _returnvalue (Game|GetPlayerController 0))
  (bind _returnvalue_2 (Pawn|GetControlledPawn _returnvalue))
  (if (Utilities|IsValid (Pawn|GetControlledPawn (Game|GetPlayerController 0)))
    ;[1 1 1] Sets player Location , player object and checks if player is alive.
    (AI|BehaviorTree|SetBlackboardValueasVector (Variables|Default|GetPlayerLocationKey) (Transformation|GetActorLocation _returnvalue_2))
    (Class|BTFunctionLibrary|SetBlackboardValueasObject (Variables|Default|GetPlayerKey) _returnvalue_2)
    (bind _asmain_character (Utilities|Casting|CastToMainCharacter (Game|GetPlayerCharacter 0)))
    (bind _returnvalue_3 (Class|MainCharacter|GetIsPlayerAlive _asmain_character))
    (Class|BTFunctionLibrary|SetBlackboardValueasBool (Variables|Default|GetIsPlayerAliveKey) _returnvalue_3)
    (else
      ;[1 1 1] If not valid, set to null
      (AI|BehaviorTree|SetBlackboardValueasVector (Variables|Default|GetPlayerLocationKey) "0, 0, 0")
      (Class|BTFunctionLibrary|SetBlackboardValueasObject (Variables|Default|GetPlayerKey)))))