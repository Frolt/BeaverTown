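; Rolling stone door Blueprint that animates its static mesh open when OpenDoorEvent fires.
; BeginPlay caches the mesh's relative rotation and location and silences the stone sound.
; The RollDoor timeline adds pitch to the cached rotation and sets local Y to its Translate value minus the cached Y, without sweep.
; A timeline event track starts the sound half a second into the clip, and Finished stops it.
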(event Custom|OpenDoorEvent
  (bind _doorloc (Variables|Default|GetDoorLoc))
  ;[1 1 1] Timeline animation that opens the door
  (bind (_direction _rotate _translate) (Timeline|RollDoor Play)
    (:Update
      (Transformation|SetRelativeRotation (Variables|Default|GetStaticMesh) (Math|Rotator|CombineRotators (Math|Rotator|MakeRotator 0.0 _rotate 0.0) (Variables|Default|GetDoorRot)) false false)
      (Transformation|SetRelativeLocation (Variables|Default|GetStaticMesh) (Math|Vector|MakeVector (.x _doorloc) (- _translate (.y _doorloc)) (.z _doorloc)) false false))
    (:Finished
      (Audio|Components|Audio|Stop (Variables|Default|GetStoneSound)))
    (:PlaySound
      (Audio|Components|Audio|Play (Variables|Default|GetStoneSound) 0.5))))

(event EventBeginPlay
  (Variables|Default|SetDoorRot (Variables|/Script/Engine.SceneComponent|GetRelativeRotation (Variables|Default|GetStaticMesh)))
  (Variables|Default|SetDoorLoc (Variables|/Script/Engine.SceneComponent|GetRelativeLocation (Variables|Default|GetStaticMesh)))
  (Audio|Components|Audio|Stop (Variables|Default|GetStoneSound)))

(fn ConstructionScript)