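; Interactable loot chest that opens and closes through ChestOpen and ChestClose events, playing and reversing a timeline.
; The timeline rotates the mesh and drives the loot light and opening sound.
; When it finishes, any loot triggers a one-time sound and particle burst, and a per-ChestNumber looted flag is saved in MainGameInstance.
; Chests already looted at BeginPlay destroy their loot effects and skip event binding.
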(event Custom|ChestOpen_Event_0
  (bind _basemesh (Variables|Default|GetBaseMesh))
  (bind _gameinstanceref (Variables|Default|GetGameInstanceREF))
  (bind _pointlight (Variables|Default|GetPointLight))
  (bind _relativerotation (Variables|/Script/Engine.SceneComponent|GetRelativeRotation _basemesh))
  (bind (_roll _pitch _yaw) (Math|Rotator|BreakRotator _relativerotation))
  (bind (_direction _openlock _lightintensity) (Timeline|Timeline_0 Play)
    (:Update
      ;[1 1 1] Opens chest lock and increase loot light with timeline
      (Transformation|SetRelativeRotation (Variables|Default|GetDerivedMesh) (Math|Rotator|CombineRotators (Math|Rotator|MakeRotator _openlock 0.0 0.0) (Math|Rotator|MakeRotator _roll _pitch (+ _yaw 9e+01))) false false)
      (if (Variables|Default|GetbHasLoot)
        (Utilities|IsValid _pointlight
          (:Is%20Valid
            (Rendering|Components|Light|SetIntensity _pointlight _lightintensity)))))
    (:Finished
      ;[1 1 1] Display loot particle and sound after chest is open
      (Rendering|SetVisibility (Variables|Default|GetLoot) false false)
      (if (and (Variables|Default|GetbHasLoot) (not (Variables|Default|GetbLooted)))
        (Audio|PlaySoundatLocation "/Game/Audio/Success.Success" (Transformation|GetWorldLocation (Variables|Default|GetLoot)))
        (Variables|Default|SetbHasLoot false)
        (Components|Activation|Activate (Variables|Default|GetChestParticles) false)
        (Variables|Default|SetbLooted true)
        ;[1 1 1] Saves chest loot status in Game Instance
        (switch int (Variables|Chest|GetChestNumber)
          (:0
            (Variables|/Script/BeaverTownDev.MainGameInstance|SetChest1Looted _gameinstanceref true))
          (:1
            (Variables|/Script/BeaverTownDev.MainGameInstance|SetChest2Looted _gameinstanceref true))
          (:2
            (Variables|/Script/BeaverTownDev.MainGameInstance|SetChest3Looted _gameinstanceref true))
          (:3
            (Variables|/Script/BeaverTownDev.MainGameInstance|SetChest4Looted _gameinstanceref true))
          (:4
            (Variables|/Script/BeaverTownDev.MainGameInstance|SetChest5Looted _gameinstanceref true)))
        ;[1 1 1] Deactivates loot after looting
        (Utilities|FlowControl|Delay 2.0)
        (Rendering|Components|Light|SetIntensity (Variables|Default|GetPointLight) 0.0)
        (Components|Activation|Deactivate (Variables|Default|GetChestParticles))))
    (:PlaySound
      (Audio|PlaySoundatLocation "/Game/Audio/DoorSound2.DoorSound2" (Transformation|GetActorLocation) "0, 0, 0" 1.0 1.0 1.0))))

(event Custom|ChestClose_Event_0
  (bind _basemesh (Variables|Default|GetBaseMesh))
  (bind _gameinstanceref (Variables|Default|GetGameInstanceREF))
  (bind _pointlight (Variables|Default|GetPointLight))
  (bind _relativerotation (Variables|/Script/Engine.SceneComponent|GetRelativeRotation _basemesh))
  (bind (_roll _pitch _yaw) (Math|Rotator|BreakRotator _relativerotation))
  (bind (_direction _openlock _lightintensity) (Timeline|Timeline_0 Reverse)
    (:Update
      ;[1 1 1] Opens chest lock and increase loot light with timeline
      (Transformation|SetRelativeRotation (Variables|Default|GetDerivedMesh) (Math|Rotator|CombineRotators (Math|Rotator|MakeRotator _openlock 0.0 0.0) (Math|Rotator|MakeRotator _roll _pitch (+ _yaw 9e+01))) false false)
      (if (Variables|Default|GetbHasLoot)
        (Utilities|IsValid _pointlight
          (:Is%20Valid
            (Rendering|Components|Light|SetIntensity _pointlight _lightintensity)))))
    (:Finished
      ;[1 1 1] Display loot particle and sound after chest is open
      (Rendering|SetVisibility (Variables|Default|GetLoot) false false)
      (if (and (Variables|Default|GetbHasLoot) (not (Variables|Default|GetbLooted)))
        (Audio|PlaySoundatLocation "/Game/Audio/Success.Success" (Transformation|GetWorldLocation (Variables|Default|GetLoot)))
        (Variables|Default|SetbHasLoot false)
        (Components|Activation|Activate (Variables|Default|GetChestParticles) false)
        (Variables|Default|SetbLooted true)
        ;[1 1 1] Saves chest loot status in Game Instance
        (switch int (Variables|Chest|GetChestNumber)
          (:0
            (Variables|/Script/BeaverTownDev.MainGameInstance|SetChest1Looted _gameinstanceref true))
          (:1
            (Variables|/Script/BeaverTownDev.MainGameInstance|SetChest2Looted _gameinstanceref true))
          (:2
            (Variables|/Script/BeaverTownDev.MainGameInstance|SetChest3Looted _gameinstanceref true))
          (:3
            (Variables|/Script/BeaverTownDev.MainGameInstance|SetChest4Looted _gameinstanceref true))
          (:4
            (Variables|/Script/BeaverTownDev.MainGameInstance|SetChest5Looted _gameinstanceref true)))
        ;[1 1 1] Deactivates loot after looting
        (Utilities|FlowControl|Delay 2.0)
        (Rendering|Components|Light|SetIntensity (Variables|Default|GetPointLight) 0.0)
        (Components|Activation|Deactivate (Variables|Default|GetChestParticles))))
    (:PlaySound
      (Audio|PlaySoundatLocation "/Game/Audio/DoorSound2.DoorSound2" (Transformation|GetActorLocation) "0, 0, 0" 1.0 1.0 1.0))))

(event EventBeginPlay
  (bind _basemesh (Variables|Default|GetBaseMesh))
  (bind _pointlight (Variables|Default|GetPointLight))
  (bind _relativerotation (Variables|/Script/Engine.SceneComponent|GetRelativeRotation _basemesh))
  (bind (_roll _pitch _yaw) (Math|Rotator|BreakRotator _relativerotation))
  (bind _asmain_game_instance (Utilities|Casting|CastToMainGameInstance (Game|GetGameInstance)))
  (Variables|Default|SetGameInstanceREF _asmain_game_instance)
  (if (Variables|Default|GetbLooted)
    ;[1 1 1] Destroys loot if looted before
    (Components|DestroyComponent (Variables|Default|GetLoot))
    (Components|DestroyComponent (Variables|Default|GetChestParticles))
    (Components|DestroyComponent (Variables|Default|GetPointLight))
    (bind (_direction _openlock _lightintensity) (Timeline|Timeline_0 SetNewTime)
      (:Update
        ;[1 1 1] Opens chest lock and increase loot light with timeline
        (Transformation|SetRelativeRotation (Variables|Default|GetDerivedMesh) (Math|Rotator|CombineRotators (Math|Rotator|MakeRotator _openlock 0.0 0.0) (Math|Rotator|MakeRotator _roll _pitch (+ _yaw 9e+01))) false false)
        (if (Variables|Default|GetbHasLoot)
          (Utilities|IsValid _pointlight
            (:Is%20Valid
              (Rendering|Components|Light|SetIntensity _pointlight _lightintensity)))))
      (:Finished
        ;[1 1 1] Display loot particle and sound after chest is open
        (Rendering|SetVisibility (Variables|Default|GetLoot) false false)
        (if (and (Variables|Default|GetbHasLoot) (not (Variables|Default|GetbLooted)))
          (Audio|PlaySoundatLocation "/Game/Audio/Success.Success" (Transformation|GetWorldLocation (Variables|Default|GetLoot)))
          (Variables|Default|SetbHasLoot false)
          (Components|Activation|Activate (Variables|Default|GetChestParticles) false)
          (Variables|Default|SetbLooted true)
          ;[1 1 1] Saves chest loot status in Game Instance
          (switch int (Variables|Chest|GetChestNumber)
            (:0
              (Variables|/Script/BeaverTownDev.MainGameInstance|SetChest1Looted (Variables|Default|GetGameInstanceREF) true))
            (:1
              (Variables|/Script/BeaverTownDev.MainGameInstance|SetChest2Looted (Variables|Default|GetGameInstanceREF) true))
            (:2
              (Variables|/Script/BeaverTownDev.MainGameInstance|SetChest3Looted (Variables|Default|GetGameInstanceREF) true))
            (:3
              (Variables|/Script/BeaverTownDev.MainGameInstance|SetChest4Looted (Variables|Default|GetGameInstanceREF) true))
            (:4
              (Variables|/Script/BeaverTownDev.MainGameInstance|SetChest5Looted (Variables|Default|GetGameInstanceREF) true)))
          ;[1 1 1] Deactivates loot after looting
          (Utilities|FlowControl|Delay 2.0)
          (Rendering|Components|Light|SetIntensity (Variables|Default|GetPointLight) 0.0)
          (Components|Activation|Deactivate (Variables|Default|GetChestParticles))))
      (:PlaySound
        (Audio|PlaySoundatLocation "/Game/Audio/DoorSound2.DoorSound2" (Transformation|GetActorLocation) "0, 0, 0" 1.0 1.0 1.0)))
    (else
      ;[1 1 1] Open and Close events from interact class
      (EventDispatchers|AssignChestOpen (delegate Custom|ChestOpen_Event_0))
      (EventDispatchers|AssignChestClose (delegate Custom|ChestClose_Event_0))
      ;[1 1 1] Displays loot of enabled
      (if (not (Variables|Default|GetbHasLoot))
        (Rendering|SetVisibility (Variables|Default|GetLoot) false false)
        (Rendering|Components|Light|SetIntensity (Variables|Default|GetPointLight) 0.0)))))

(fn ConstructionScript)