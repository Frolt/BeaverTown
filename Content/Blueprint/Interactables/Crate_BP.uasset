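; Breakable crate interactable that can drop a red crystal pickup when destroyed.
; At BeginPlay it binds a handler to its CrateOpen event, which checks GetIsBroken on each call.
; An unbroken crate only plays a damage sound.
; A broken one plays another sound, spawns the pickup at the mesh's SpawnLocation socket if RandomSpawn converts to true, then destroys itself.
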(event Custom|CrateOpen_Event_0
  (bind _returnvalue (Transformation|GetActorLocation))
  (bind _returnvalue_2 (Class|Crate|GetIsBroken))
  (if _returnvalue_2
    ;[1 1 1] Spawns crystal when crate is destroyed
    (Audio|PlaySoundatLocation "/Game/Audio/CrateDamage.CrateDamage" _returnvalue)
    (if (Math|Conversions|ToBoolean(Integer) (Variables|Default|GetRandomSpawn))
      (Game|SpawnActorfromClass "/Game/Blueprint/Pickups/PickupCrystalRed.PickupCrystalRed_C" (Math|Transform|MakeTransform (Transformation|GetSocketLocation (Variables|Default|GetCrate) "SpawnLocation") (Transformation|GetActorRotation) "1,1,1") "Undefined" 0 0)
      (Actor|DestroyActor)
      (else
        (Actor|DestroyActor)))
    (else
      (Audio|PlaySoundatLocation "/Game/Audio/CreateDamage2.CreateDamage2" _returnvalue))))

(event EventBeginPlay
  (EventDispatchers|AssignCrateOpen (delegate Custom|CrateOpen_Event_0)))

(fn ConstructionScript)