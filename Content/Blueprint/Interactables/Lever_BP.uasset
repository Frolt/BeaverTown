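; Lever interactable actor that toggles an Active state and animates a pull when opened or closed.
; On BeginPlay it binds to its own LeverOpen and LeverClose dispatchers, each setting Active and playing a sound at the actor.
; Opening plays a timeline that rolls the lever mesh relative to the base mesh's rotation with a yaw offset; closing reverses that timeline.
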(event Custom|LeverClose_Event_0
  (bind _basemesh (Variables|Default|GetBaseMesh))
  (bind _relativerotation (Variables|/Script/Engine.SceneComponent|GetRelativeRotation _basemesh))
  (bind (_roll _pitch _yaw) (Math|Rotator|BreakRotator _relativerotation))
  (Variables|Default|SetActive false)
  (Audio|PlaySoundatLocation "/Game/Audio/PickupSound.PickupSound" (Transformation|GetActorLocation))
  ;[1 1 1] Pull lever with timeline
  (bind _lever_roll (Timeline|Lever%20Timeline Reverse)
    (:Update
      (Transformation|SetRelativeRotation (Variables|Default|Getlever) (Math|Rotator|CombineRotators (Math|Rotator|MakeRotator _lever_roll 0.0 0.0) (Math|Rotator|MakeRotator _roll _pitch (+ _yaw -9e+01))) false false))))

(event Custom|LeverOpen_Event_0
  (bind _basemesh (Variables|Default|GetBaseMesh))
  (bind _relativerotation (Variables|/Script/Engine.SceneComponent|GetRelativeRotation _basemesh))
  (bind (_roll _pitch _yaw) (Math|Rotator|BreakRotator _relativerotation))
  (Variables|Default|SetActive true)
  (Audio|PlaySoundatLocation "/Game/Audio/PickupSound.PickupSound" (Transformation|GetActorLocation))
  ;[1 1 1] Pull lever with timeline
  (bind _lever_roll (Timeline|Lever%20Timeline Play)
    (:Update
      (Transformation|SetRelativeRotation (Variables|Default|Getlever) (Math|Rotator|CombineRotators (Math|Rotator|MakeRotator _lever_roll 0.0 0.0) (Math|Rotator|MakeRotator _roll _pitch (+ _yaw -9e+01))) false false))))

(event EventBeginPlay
  (EventDispatchers|AssignLeverOpen (delegate Custom|LeverOpen_Event_0))
  (EventDispatchers|AssignLeverClose (delegate Custom|LeverClose_Event_0)))

(fn ConstructionScript)