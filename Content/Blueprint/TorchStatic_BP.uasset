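; Static torch actor that can start lit or extinguished and switches between the two through Ignite and Extinguish.
; Both functions toggle fire particles, looping sound and the head material, then drive a timeline forward or backward to fade light intensity and emissive strength.
; Igniting can also start a referenced fire sequence when enabled.
; The timeline creates a dynamic material instance on every update.
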(event OnAudioFinished(FireSound)
  (if (Variables|Default|GetbIsLit)
    (Audio|Components|Audio|Play (Variables|Default|GetFireSound) 0.0)))

(event Custom|Decrease%20Light
  ;[1 1 1] LIght Intensity
  (bind (_direction _light_intensity _material_emission) (Timeline|Change%20Light Reverse)
    (:Update
      (Rendering|Components|Light|SetIntensity (Variables|Default|GetTorchLight) _light_intensity)
      (bind _returnvalue (Rendering|Material|CreateDynamicMaterialInstance (Variables|Default|GetTorchMesh) 2 0 :!class /Script/Engine.PrimitiveComponent))
      (Rendering|Material|SetScalarParameterValue _returnvalue "Emissive strength" _material_emission :!class /Script/Engine.MaterialInstanceDynamic))))

(event Custom|Increase%20light
  ;[1 1 1] LIght Intensity
  (bind (_direction _light_intensity _material_emission) (Timeline|Change%20Light Play)
    (:Update
      (Rendering|Components|Light|SetIntensity (Variables|Default|GetTorchLight) _light_intensity)
      (bind _returnvalue (Rendering|Material|CreateDynamicMaterialInstance (Variables|Default|GetTorchMesh) 2 0 :!class /Script/Engine.PrimitiveComponent))
      (Rendering|Material|SetScalarParameterValue _returnvalue "Emissive strength" _material_emission :!class /Script/Engine.MaterialInstanceDynamic))))

(event EventBeginPlay
  ;[1 1 1] Can start in Ignite or extinguish modus
  (if (Variables|Default|GetbIsLit)
    (CallFunction|Ignite)
    (else
      (CallFunction|Extinguish))))

(fn ConstructionScript)

(fn Ignite
  (bind _firesequenceref (Variables|TorchStatic|GetFireSequenceRef))
  ;[1 1 1] Ignites torch according to settings
  (Components|Activation|Activate (Variables|Default|GetFireParticles) false)
  (Variables|Default|SetbIsLit true)
  (Rendering|Material|SetMaterial (Variables|Default|GetTorchMesh) 2 (Variables|TorchStatic|GetMaterial%20Instance))
  (CallFunction|IncreaseLight)
  (if (Variables|Default|GetbIsLit)
    (Audio|Components|Audio|Play (Variables|Default|GetFireSound) 0.0)
    (if (Variables|TorchStatic|GetTriggerFireSequence)
      (if (Utilities|IsValid _firesequenceref)
        (Default|BeginFire _firesequenceref)))))

(fn Extinguish
  ;[1 1 1] Extinguish torch
  (Components|Activation|Deactivate (Variables|Default|GetFireParticles))
  (Variables|Default|SetbIsLit false)
  (Rendering|Material|SetMaterial (Variables|Default|GetTorchMesh) 2 "/Game/Materials/M_PaintedWood.M_PaintedWood")
  (CallFunction|DecreaseLight)
  (Audio|Components|Audio|Stop (Variables|Default|GetFireSound)))