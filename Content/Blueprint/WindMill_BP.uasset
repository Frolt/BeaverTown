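; Windmill actor Blueprint that continuously spins its Mill component.
; On BeginPlay it starts the BladeSpin timeline, which drives a roll rotation combined with the stored Rotation and applies it as the Mill's relative rotation each update.
; When the timeline finishes it calls StartWindmill again to loop the spin.
; The stored Rotation is captured from the Mill right after the first start call.
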(event Custom|StartWindmill
  ;[1 1 1] Animates windmill with timeline
  (bind _newtrack_0 (Timeline|BladeSpin Play)
    (:Update
      (Transformation|SetRelativeRotation (Variables|Default|GetMill) (Math|Rotator|CombineRotators (Math|Rotator|MakeRotator _newtrack_0 0.0 0.0) (Variables|Default|GetRotation)) false false))
    (:Finished
      (CallFunction|StartWindmill))))

(event EventBeginPlay
  (CallFunction|StartWindmill)
  (Variables|Default|SetRotation (Variables|/Script/Engine.SceneComponent|GetRelativeRotation (Variables|Default|GetMill))))

(fn ConstructionScript)