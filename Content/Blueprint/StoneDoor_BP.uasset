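; Stone door actor that opens and closes according to a referenced lever.
; BeginPlay caches the mesh's relative location, and Tick polls the lever's IsOpenEvent flag to play or reverse the DoorOpenClose timeline.
; Timeline updates keep the cached X and Y and set Z to the Lower track value minus the cached Z.
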(event EventBeginPlay
  (Variables|Default|SetDoorLocation (Variables|/Script/Engine.SceneComponent|GetRelativeLocation (Variables|Default|GetStaticMesh))))

(event EventTick
  (params (DeltaSeconds :type Float%20%28single-precision%29))
  (bind _doorlocation (Variables|Default|GetDoorLocation))
  ;[1 1 1] Lever can open the door
  (if (Variables|/Script/BeaverTownDev.Interact|GetbIsOpenEvent (Variables|Default|GetLeverREF))
    ;[1 1 1] Timeline animation that opens the door
    (bind _lower (Timeline|DoorOpen/Close Play)
      (:Update
        (Transformation|SetRelativeLocation (Variables|Default|GetStaticMesh) (Math|Vector|MakeVector (.x _doorlocation) (.y _doorlocation) (- _lower (.z _doorlocation))) false false)))
    (else
      (Timeline|DoorOpen/Close Reverse))))

(fn ConstructionScript)