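; Raft Blueprint that carries four static torches as child actors and turns off their collision when play begins.
; On BeginPlay it casts each torch's child actor to TorchStatic_BP, then sets the static mesh component found on each to ignore all collision channels.
; All four casts run before any change, so one failed cast leaves every torch's collision untouched.
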(event EventBeginPlay
  ;[1 1 1] Turns off collision on Torches
  (bind _astorch_static_bp (Utilities|Casting|CastToTorchStatic_BP (Variables|/Script/Engine.ChildActorComponent|GetChildActor (Variables|Default|GetTorch2))))
  (bind _astorch_static_bp_2 (Utilities|Casting|CastToTorchStatic_BP (Variables|/Script/Engine.ChildActorComponent|GetChildActor (Variables|Default|GetTorch3))))
  (bind _astorch_static_bp_3 (Utilities|Casting|CastToTorchStatic_BP (Variables|/Script/Engine.ChildActorComponent|GetChildActor (Variables|Default|GetTorch4))))
  (bind _astorch_static_bp_4 (Utilities|Casting|CastToTorchStatic_BP (Variables|/Script/Engine.ChildActorComponent|GetChildActor (Variables|Default|GetTorch1))))
  (Collision|SetCollisionResponsetoAllChannels (Actor|GetComponentbyClass _astorch_static_bp "/Script/Engine.StaticMeshComponent") "ECR_Ignore")
  (Collision|SetCollisionResponsetoAllChannels (Actor|GetComponentbyClass _astorch_static_bp_2 "/Script/Engine.StaticMeshComponent") "ECR_Ignore")
  (Collision|SetCollisionResponsetoAllChannels (Actor|GetComponentbyClass _astorch_static_bp_3 "/Script/Engine.StaticMeshComponent") "ECR_Ignore")
  (Collision|SetCollisionResponsetoAllChannels (Actor|GetComponentbyClass _astorch_static_bp_4 "/Script/Engine.StaticMeshComponent") "ECR_Ignore"))

(fn ConstructionScript)